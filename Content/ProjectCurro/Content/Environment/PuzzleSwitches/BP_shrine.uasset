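; Shrine puzzle actor where the player deposits collected pickups as orbs that fly to a bird statue.
; An EventHandler-bound capture attempt, allowed inside the trigger, spawns randomly angled ShrineOrbs from the pickup count, then zeroes it.
; Tick feeds orbs through three arrays: queued on a cooldown, drifting outward, then homing on the statue until PickupCollision destroys them.
; The shrine-captured and UI fade calls are never executed.
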(event OnComponentBeginOverlap(PickupCollision)
  (params (OtherActor :type Actor%20Object%20Reference) (OtherComp :type Primitive%20Component%20Object%20Reference) (OtherBodyIndex :type Integer) (bFromSweep :type Boolean) (SweepResult :type Hit%20Result%20Structure%20%28by%20ref%29))
  (bind _asshrine_orb (Utilities|Casting|CastToShrineOrb OtherActor))
  (bind _returnvalue (Utilities|Array|RemoveItem (Variables|Default|GetDepositOrbs) _asshrine_orb))
  (if _returnvalue
    (Actor|DestroyActor _asshrine_orb)))

(event OnComponentBeginOverlap(CurroCollision)
  (params (OtherActor :type Actor%20Object%20Reference) (OtherComp :type Primitive%20Component%20Object%20Reference) (OtherBodyIndex :type Integer) (bFromSweep :type Boolean) (SweepResult :type Hit%20Result%20Structure%20%28by%20ref%29))
  (if (== OtherActor (Game|GetPlayerCharacter 0))
    (Utilities|Casting|CastToPawn_Curro OtherActor)
    (Variables|Default|SetCanCapture true)
    (Development|SetHiddeninGame (Variables|Default|GetTriggerIndicator) false true)))

(event OnComponentEndOverlap(CurroCollision)
  (params (OtherActor :type Actor%20Object%20Reference) (OtherComp :type Primitive%20Component%20Object%20Reference) (OtherBodyIndex :type Integer))
  (if (== (Game|GetPlayerCharacter 0) OtherActor)
    (Utilities|Casting|CastToPawn_Curro OtherActor)
    (Variables|Default|SetCanCapture false)
    (Development|SetHiddeninGame (Variables|Default|GetTriggerIndicator) true true)))

(event Custom|AttemptCapture
  (params (Capturer :type Pawn%20Curro%20Object%20Reference))
  ;[1 1 1] Attempt Capture
  (if (Variables|Default|GetCanCapture)
    (bind _count (Default|GetPickupCount Capturer))
    (for _index (range 0 _count)
      (Variables|Default|SetCapturerUpVec (Transformation|GetActorUpVector Capturer))
      (bind _returnvalue (Game|SpawnActorfromClass "/Game/ProjectCurro/Content/Objects/ShrineOrb.ShrineOrb_C" (Math|Conversions|ToTransform(Vector) (Transformation|GetActorLocation Capturer)) false 0 0))
      (Default|SetDirectionVec _returnvalue (Math|Vector|RotateVector (Variables|Default|GetCapturerUpVec) (Class|KismetMathLibrary|MakeRot (Math|Random|RandomFloatinRange -9e+01 9e+01) (Math|Random|RandomFloatinRange 45.0 -15.0) 0.0)))
      (Default|SetOriginLoc _returnvalue (Transformation|GetActorLocation _returnvalue))
      (Utilities|Array|Add (Variables|Default|GetOrbArray) _returnvalue))
    (Variables|Default|SetShrineState "NewEnumerator0")
    (Default|SetPickupCount Capturer)))

(event EventBeginPlay
  ;[1 1 1] Get Event Handler
  (bind _outactors (Actor|GetAllActorsOfClass "/Game/ProjectCurro/Content/UI/EventHandler.EventHandler_C"))
  (for _array_element _outactors
    (bind _output_get (Variables|Default|SetEventHandleRef _array_element))
    (EventDispatchers|BindEventtoAttemptShrineCapture _output_get (delegate Custom|AttemptCapture))))

(event EventTick
  (params (DeltaSeconds :type Float%20%28single-precision%29))
  ;[1 1 1] Attempt Capture
  (switch Utilities|FlowControl|Switch|SwitchonShrineState (Variables|Default|GetShrineState)
    (:NewEnumerator0
      (Utilities|FlowControl|Sequence
        (:then_0
          (bind _output_get (Variables|Default|SetCooldown (- (Variables|Default|GetCooldown) DeltaSeconds)))
          (if (<= _output_get 0.0)
            (CallFunction|MoveOrbs)
            (Variables|Default|SetCooldown 0.3)))
        (:then_1
          (CallFunction|ReleasePickups DeltaSeconds))
        (:then_2
          (CallFunction|DepositPickups DeltaSeconds))))))

(fn ConstructionScript)

(fn ReleasePickups
  (params (dt :type Float%20%28single-precision%29))
  (for (_ _array_index) (Variables|Default|GetReleaseOrbs)
    (Variables|Default|SetCurrentIndex _array_index)
    (bind _vec (Default|GetDirectionVec (Utilities|Array|Get(acopy) (Variables|Default|GetReleaseOrbs) (Variables|Default|GetCurrentIndex))))
    (Transformation|SetActorLocation (Utilities|Array|Get(acopy) (Variables|Default|GetReleaseOrbs) (Variables|Default|GetCurrentIndex)) (+ (Transformation|GetActorLocation (Utilities|Array|Get(acopy) (Variables|Default|GetReleaseOrbs) (Variables|Default|GetCurrentIndex))) (* _vec (* dt (LocalVariables|GetReleaseScalar)))) false)
    (bind _vec_2 (Default|GetOriginLoc (Utilities|Array|Get(acopy) (Variables|Default|GetReleaseOrbs) (Variables|Default|GetCurrentIndex))))
    (if (>= (Math|Vector|VectorLength (- _vec_2 (Transformation|GetActorLocation (Utilities|Array|Get(acopy) (Variables|Default|GetReleaseOrbs) (Variables|Default|GetCurrentIndex))))) (Math|Random|RandomFloatinRange 1.3e+02 1.9e+02))
      (Utilities|Array|Add (Variables|Default|GetDepositOrbs) (Utilities|Array|Get(acopy) (Variables|Default|GetReleaseOrbs) (Variables|Default|GetCurrentIndex)))
      (Utilities|Array|RemoveIndex (Variables|Default|GetReleaseOrbs) (Variables|Default|GetCurrentIndex)))))

(fn DepositPickups
  (params (dt :type Float%20%28single-precision%29))
  (LocalVariables|SetTargetLoc (+ (Transformation|GetWorldLocation (Variables|Default|GetBirdStatue)) "0, 0,100.000000"))
  (if (!= (Utilities|Array|Length (Variables|Default|GetDepositOrbs)) 0)
    (for _array_element (Variables|Default|GetDepositOrbs)
      (Transformation|SetActorLocation _array_element (+ (Transformation|GetActorLocation _array_element) (* (Class|KismetMathLibrary|GetDirectionVector (Transformation|GetActorLocation _array_element) (LocalVariables|GetTargetLoc)) (* dt (LocalVariables|GetDepositScalar)))) false))))

(fn MoveOrbs
  (for _array_element (Variables|Default|GetOrbArray)
    (Utilities|Array|RemoveItem (Variables|Default|GetOrbArray) _array_element)
    (Utilities|Array|Add (Variables|Default|GetReleaseOrbs) _array_element)))