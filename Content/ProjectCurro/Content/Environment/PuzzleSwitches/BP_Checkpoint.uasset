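; Checkpoint actor that registers itself with the Pawn_Curro pawn when that pawn enters its trigger.
; BeginPlay sizes the TriggerBox from the TriggerExtents variable, and overlaps by any other actor type are ignored.
; GetSpawnPoint exposes the world location of the SpawnPoint component, supplying a position only, without rotation.
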(event `self.ReceiveBeginPlay`
  (`BoxComponent.SetBoxExtent` (`self.TriggerBox`) (`self.TriggerExtents`) true))

(event `self.TriggerBox.OnComponentBeginOverlap`
  (params (OtherActor :type "Actor Object Reference") (OtherComp :type "PrimitiveComponent Object Reference") (OtherBodyIndex :type Integer) (bFromSweep :type Boolean) (SweepResult :type "HitResult Structure (by ref)"))
  (bind _aspawn_curro (cast `/Game/ProjectCurro/Content/Characters/Curro/Pawn_Curro` OtherActor))
  (`/Game/ProjectCurro/Content/Characters/Curro/Pawn_Curro.SetCheckpoint` _aspawn_curro self))

(event `self.ReceiveTick`
  (params (DeltaSeconds :type "Float (single-precision)")))

(fn `GetSpawnPoint`
  (returns (Position :type "Vector Structure"))
  (return (`SceneComponent.K2_GetComponentLocation` (`self.SpawnPoint`))))

(fn `UserConstructionScript`)