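; World tutorial prompt that shows a stack of text materials on a billboard, revealed while Pawn_Curro is inside its interaction sphere.
; On BeginPlay it displays the last material in TextArray and binds InteractTutorial to every EventHandler actor.
; Each interaction while in range removes that last entry and shows the new last one, with no empty-array guard.
; It also stores a checkpoint through a simple getter and setter.
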(event `self.ReceiveBeginPlay`
  (`self.RemovePreviousMaterial`)
  (`self.GetAndSetLatestMaterial`)
  (bind _outactors (`GameplayStatics.GetAllActorsOfClass` "/Game/ProjectCurro/Content/UI/EventHandler.EventHandler_C"))
  (for _array_element _outactors
    (bind _output_get (set `self.EventHandleRef` _array_element))
    (add `/Game/ProjectCurro/Content/UI/EventHandler.InteractTutorial` _output_get (delegate `InteractTutorial`))))

(event `InteractTutorial`
  (bind _textarray (`self.TextArray`))
  (if (`self.canInteract`)
    (`self.RemovePreviousMaterial`)
    (`KismetArrayLibrary.Array_Remove` _textarray (- (`KismetArrayLibrary.Array_Length` _textarray) 1))
    (`self.GetAndSetLatestMaterial`)))

(event `self.InteractionSphere.OnComponentBeginOverlap`
  (params (OtherActor :type "Actor Object Reference") (OtherComp :type "PrimitiveComponent Object Reference") (OtherBodyIndex :type Integer) (bFromSweep :type Boolean) (SweepResult :type "HitResult Structure (by ref)"))
  (cast `/Game/ProjectCurro/Content/Characters/Curro/Pawn_Curro` OtherActor)
  (set `self.canInteract` true)
  (`SceneComponent.SetHiddenInGame` (`self.TextBox`) (not (`self.canInteract`)) true :!label _label))

(event `self.InteractionSphere.OnComponentEndOverlap`
  (params (OtherActor :type "Actor Object Reference") (OtherComp :type "PrimitiveComponent Object Reference") (OtherBodyIndex :type Integer))
  (cast `/Game/ProjectCurro/Content/Characters/Curro/Pawn_Curro` OtherActor)
  (set `self.canInteract` false)
  (goto _label))

(fn `GetAndSetLatestMaterial`
  (bind _textarray (`self.TextArray`))
  (`MaterialBillboardComponent.AddElement` (`self.TextBox`) (`KismetArrayLibrary.Array_Get` _textarray (- (`KismetArrayLibrary.Array_Length` _textarray) 1)) null false 80.0 250.0 null))

(fn `GetCheckpoint`
  (returns (NewParam :type "/Game/ProjectCurro/Content/Environment/PuzzleSwitches/BP_Checkpoint Object Reference"))
  (return (`self.myCheckpoint`)))

(fn `RemovePreviousMaterial`
  (`KismetArrayLibrary.Array_Clear` (`MaterialBillboardComponent.Elements` (`self.TextBox`))))

(fn `SetCheckpoint`
  (params (`new checkpoint` :type "/Game/ProjectCurro/Content/Environment/PuzzleSwitches/BP_Checkpoint Object Reference"))
  (set `self.myCheckpoint` `new checkpoint`))

(fn `UserConstructionScript`)