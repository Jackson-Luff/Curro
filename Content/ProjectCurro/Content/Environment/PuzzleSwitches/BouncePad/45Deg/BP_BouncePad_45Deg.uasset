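; A 45-degree bounce pad from the puzzle switch environment set that launches any Pawn_Base overlapping its BounceMesh.
; ApplyBounce scales a normalized Z direction from the mesh's world rotation by BounceStrength and adds the pawn's negated velocity.
; LaunchCharacter applies the result additively, so the negated term cancels incoming motion and the exit velocity depends only on pad orientation and strength.
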(event `self.ReceiveBeginPlay`)

(event `self.ReceiveActorBeginOverlap`
  (params (OtherActor :type "Actor Object Reference")))

(event `self.ReceiveTick`
  (params (DeltaSeconds :type "Float (single-precision)")))

(event `self.bounceMesh.OnComponentBeginOverlap`
  (params (OtherActor :type "Actor Object Reference") (OtherComp :type "PrimitiveComponent Object Reference") (OtherBodyIndex :type Integer) (bFromSweep :type Boolean) (SweepResult :type "HitResult Structure (by ref)"))
  (bind _aspawn_base (cast `/Game/ProjectCurro/Content/Characters/Pawn_Base` OtherActor))
  (bind _velocity (`self.ApplyBounce` (`self.BounceStrength`) (`self.GetVelocity` _aspawn_base)))
  (`Character.LaunchCharacter` _aspawn_base _velocity false false))

(fn `ApplyBounce`
  (params (Strength :type "Float (double-precision)") (PawnVelocity :type "Vector Structure"))
  (returns (Velocity :type "Vector Structure"))
  (return (+ (* (`KismetMathLibrary.Normal` (`.Z` (`KismetMathLibrary.BreakRotIntoAxes` (`SceneComponent.K2_GetComponentRotation` (`self.bounceMesh`))))) Strength) (* (-1.0 -1.0 -1.0) PawnVelocity))))

(fn `UserConstructionScript`)