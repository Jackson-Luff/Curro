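; Out-of-bounds trigger volume that reports a player death when a Curro or bird pawn enters it.
; On BeginPlay it sizes its box from the Extent variable and caches the first EventHandler actor in the level.
; Box overlaps call the handler's CallPlayerDied, with a boolean that is false for Pawn_Curro and true for Pawn_Animal_Bird; other actors are ignored.
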(event `self.ReceiveBeginPlay`
  (`BoxComponent.SetBoxExtent` (`self.Box`) (`self.Extent`) true)
  (bind _outactors (`GameplayStatics.GetAllActorsOfClass` "/Game/ProjectCurro/Content/UI/EventHandler.EventHandler_C"))
  (set `self.EventHandlerRef` (`KismetArrayLibrary.Array_Get` _outactors)))

(event `self.ReceiveActorBeginOverlap`
  (params (OtherActor :type "Actor Object Reference")))

(event `self.ReceiveTick`
  (params (DeltaSeconds :type "Float (single-precision)")))

(event `self.Box.OnComponentBeginOverlap`
  (params (OtherActor :type "Actor Object Reference") (OtherComp :type "PrimitiveComponent Object Reference") (OtherBodyIndex :type Integer) (bFromSweep :type Boolean) (SweepResult :type "HitResult Structure (by ref)"))
  (cast `/Game/ProjectCurro/Content/Characters/Curro/Pawn_Curro` OtherActor
    (:`then`
      (`/Game/ProjectCurro/Content/UI/EventHandler.PlayerDied` (`self.EventHandlerRef`) false))
    (:`CastFailed`
      (cast `/Game/ProjectCurro/Content/Characters/Bird/Pawn_Animal_Bird` OtherActor)
      (`/Game/ProjectCurro/Content/UI/EventHandler.PlayerDied` (`self.EventHandlerRef`) true))))

(fn `UserConstructionScript`)